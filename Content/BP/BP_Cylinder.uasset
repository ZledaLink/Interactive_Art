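; Reactive cylinder prop with an arrow that responds each tick to its distance from a target actor.
; Distance feeds a curve and power function for the cylinder's smoothed height, which drives its tint.
; Within range, the arrow eases to face the target, grows and lifts, while its tint follows distance.
; Two slider Blueprints are polled every tick to scale height and adjust curve power and both ranges.
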(event `self.ReceiveBeginPlay`
  (bind _returnvalue (`PrimitiveComponent.CreateDynamicMaterialInstance` (`self.Cylinder`) 0 "/Game/Megascans/Surfaces/Scratched_Polyvinyl_Carbonate_Plastic_sccnbdnp/MI_White.MI_White" "None"))
  (set `self.Mat_Cylinder` _returnvalue)
  (bind _returnvalue_2 (`PrimitiveComponent.CreateDynamicMaterialInstance` (`self.SM_Arrow`) 0 "/Game/Megascans/Surfaces/Scratched_Polyvinyl_Carbonate_Plastic_sccnbdnp/MI_Arrow.MI_Arrow" "None"))
  (set `self.Mat_Arrow` _returnvalue_2))

(event `self.ReceiveTick`
  (params (DeltaSeconds :type "Float (single-precision)"))
  (bind _distance (`self.CalculateDistanceAngle`))
  (set `self.DeltaSeconds` DeltaSeconds)
  (`self.ApplySliderValues`)
  (set `self.CurrentDistance` _distance)
  (set `self.RotationEnabled` (< _distance (* (`self.MaxRotRrange`) (`self.RotScalar`))))
  ;[1 0 0.08432] Cylinder Tick
  (`self.SetHeightZ`)
  (`self.SetColorCylinder`)
  ;[1 0 0.08432] Arrow Tick
  (`self.SetRotationZ`)
  (`self.SetScaleHeight`)
  (`self.SetCololrArrow`))

(event `SetHeightZ`
  ;[1 0 0.08283] Cylinder Height Set RotationZ
  (bind _output_get (set `self.CurrentHeight` (`KismetMathLibrary.FInterpTo` (`self.CurrentHeight`) (`self.CustomInterp` (`self.CalculateDistanceAngle`) (* (`self.MaxRange`) (`self.RangeSclar`)) (`self.Power`) (* (`self.Max Height`) (`self.HeightScalar`))) (`self.DeltaSeconds`) 8.0)))
  (`SceneComponent.K2_SetRelativeLocation` (`self.Cylinder`) (`KismetMathLibrary.MakeVector` 0.0 0.0 _output_get) false false))

(event `SetRotationZ`
  ;[0.7917 0.7814 0.7732] Arrow Rotaton, Scale & Height
  ;;[1 0 0.08228] Set RotationZ
  (bind _output_get (set `self.CurrentRotation` (`KismetMathLibrary.FInterpTo` (`self.CurrentRotation`) (select `bool` (`self.RotationEnabled`) :`false` 90.0 :`true` (`.Rotation Z` (`self.CalculateDistanceAngle`))) (`self.DeltaSeconds`) 4.0)))
  (`SceneComponent.K2_SetWorldRotation` (`self.SM_Arrow`) (`KismetMathLibrary.MakeRotator` 0.0 0.0 _output_get) false false))

(event `SetScaleHeight`
  (bind _rotationenabled (`self.RotationEnabled`))
  ;[0.7917 0.7814 0.7732] Arrow Rotaton, Scale & Height
  ;;[1 0 0.07819] Set Scale Height
  (`SceneComponent.SetRelativeScale3D` (`self.SM_Arrow`) (select `bool` _rotationenabled :`false` (0.8 0.8 0.8) :`true` (1.2 1.2 1.2) :!type "Vector Structure"))
  (`SceneComponent.K2_SetRelativeLocation` (`self.SM_Arrow`) (select `bool` _rotationenabled :`true` (0.0 0.0 5.0) :!type "Vector Structure") false false))

(fn `ApplySliderValues`
  (bind _value (`/Game/BP/BP_Slider.GetSliderValue` (`self.BP_Slider_Height`) true))
  (set `self.HeightScalar` _value)
  (bind _value_2 (`/Game/BP/BP_Slider.GetSliderValue` (`self.BP_Slider_Contrast`) false))
  (set `self.Power` (`KismetMathLibrary.MapRangeClamped` _value_2 0.0 1.0 1.0 2.0))
  (set `self.RotScalar` (`KismetMathLibrary.MapRangeClamped` _value_2 0.0 1.0 1.0 1.25))
  (set `self.RangeSclar` (`KismetMathLibrary.MapRangeClamped` _value_2 0.0 1.0 1.0 1.2)))

(fn `CalculateDistanceAngle`
  (returns (Distance :type "Float (double-precision)") (`Rotation Z` :type "Float (double-precision)"))
  (bind _returnvalue (- (`self.K2_GetActorLocation` (`self.TargetActor`)) (`self.K2_GetActorLocation`)))
  ;[0.9671 0.9899 1] Calculate Distance Angle
  (return (`KismetMathLibrary.VSize` _returnvalue) (.yaw (`KismetMathLibrary.MakeRotFromX` (`KismetMathLibrary.Normal` _returnvalue 0.1)))))

(fn `CustomInterp`
  (params (InDistance :type "Float (double-precision)") (MaxRange :type "Float (double-precision)") (Power :type "Float (double-precision)") (MaxHeight :type "Float (double-precision)"))
  (returns (OutInterp :type "Float (double-precision)"))
  ;[1 1 1] Custom Interp
  (return (* (`KismetMathLibrary.MultiplyMultiply_FloatFloat` (`CurveFloat.GetFloatValue` (`self.CurveAsset`) (`KismetMathLibrary.MapRangeClamped` InDistance 0.0 MaxRange 0.0 1.0)) Power) MaxHeight)))

(fn `SetCololrArrow`
  ;[1 1 1] Set Color Arrow
  (`MaterialInstanceDynamic.SetVectorParameterValue` (`self.Mat_Arrow`) "Albedo Tint" (`KismetMathLibrary.LinearColorLerp` (struct :`R` 1.0 :`G` 1.0 :`B` 1.0 :`A` 1.0) (struct :`R` 5.0 :`G` 0.594909 :`B` 0.246415 :`A` 1.0) (`KismetMathLibrary.MapRangeClamped` (`self.CurrentDistance`) 0.0 (+ (`self.MaxRotRrange`) 200.0) 1.0))))

(fn `SetColorCylinder`
  ;[1 1 1] Set Color Cylinder
  (`MaterialInstanceDynamic.SetVectorParameterValue` (`self.Mat_Cylinder`) "Albedo Tint" (`KismetMathLibrary.LinearColorLerp` (struct :`R` 1.0 :`G` 1.0 :`B` 1.0 :`A` 1.0) (struct :`R` 6.0 :`G` 0.713891 :`B` 0.295698 :`A` 1.0) (`KismetMathLibrary.MapRangeClamped` (`self.CurrentHeight`) 0.0 350.0 0.0 1.0))))

(fn `UserConstructionScript`)